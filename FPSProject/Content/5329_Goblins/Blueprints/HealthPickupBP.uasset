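; HealthPickupBP is a health pickup actor that restores a fixed amount of health to the player.
; Any overlap with its capsule plays a sound, calls the pickup logic and removes the particle component, with no check on the overlapping actor.
; The logic, gated by a validity check, destroys the actor, then casts player character 0 to PlayerBP and adds to CurrentHealth without clamping.
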(event `HealthPickup_Logic`
  (bind _returnvalue (`GameplayStatics.GetPlayerCharacter` 0))
  (`/Engine/EditorBlueprintResources/StandardMacros.IsValid` null
    (:`Is Valid`
      (`self.K2_DestroyActor`)
      (bind _asplayer_bp (cast `/Game/5329_Goblins/Blueprints/PlayerBP` _returnvalue))
      (set `/Game/5329_Goblins/Blueprints/PlayerBP.Current Health` (+ (`/Game/5329_Goblins/Blueprints/PlayerBP.Current Health` _asplayer_bp) 20.0) _asplayer_bp)
      (cast `/Game/5329_Goblins/Blueprints/PlayerBP` _returnvalue))))

(event `self.Capsule.OnComponentBeginOverlap`
  (params (OverlappedComponent :type "PrimitiveComponent Object Reference") (OtherActor :type "Actor Object Reference") (OtherComp :type "PrimitiveComponent Object Reference") (OtherBodyIndex :type Integer) (bFromSweep :type Boolean) (SweepResult :type "HitResult Structure (by ref)"))
  (`GameplayStatics.PlaySoundAtLocation` "/Engine/EditorSounds/GamePreview/EjectFromPlayer_Cue.EjectFromPlayer_Cue" (`self.K2_GetActorLocation`))
  (`self.HealthPickup_Logic`)
  (`/Engine/EditorBlueprintResources/StandardMacros.IsValid` null
    (:`Is Valid`
      (`ActorComponent.K2_DestroyComponent` (`self.ParticleSystem`)))))

(fn `UserConstructionScript`)