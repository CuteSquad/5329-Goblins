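; ExplodingBarrelBP is a barrel actor that explodes when its capsule registers a hit.
; The hit spawns a scaled-up explosion particle effect, applies radial damage at the barrel's location and fires a RadialForce impulse.
; The explosion sound plays at the world origin rather than at the barrel.
; Only the Barrel component is destroyed afterwards, and the hit event has no guard against firing again.
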(event `self.Capsule.OnComponentHit`
  (params (HitComponent :type "PrimitiveComponent Object Reference") (OtherActor :type "Actor Object Reference") (OtherComp :type "PrimitiveComponent Object Reference") (NormalImpulse :type "Vector Structure") (Hit :type "HitResult Structure (by ref)"))
  (`GameplayStatics.SpawnEmitterAtLocation` "/Game/StarterContent/Particles/P_Explosion.P_Explosion" (`SceneComponent.K2_GetComponentLocation` (`self.Barrel`)) (struct) (5.0 5.0 5.0))
  (`GameplayStatics.PlaySoundAtLocation` "/Game/StarterContent/Audio/Explosion01.Explosion01")
  (`GameplayStatics.ApplyRadialDamage` 5.0 (`SceneComponent.K2_GetComponentLocation` (`self.Barrel`)) 50.0)
  (`RadialForceComponent.FireImpulse` (`self.RadialForce`))
  (`ActorComponent.K2_DestroyComponent` (`self.Barrel`)))

(fn `UserConstructionScript`)